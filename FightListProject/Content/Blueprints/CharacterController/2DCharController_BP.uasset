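; A 2D side-scrolling character controller Blueprint that moves a flipbook-animated character along the world X axis and lets it jump.
; The horizontal input axis feeds movement input and switches the sprite between idle and run flipbooks.
; Non-zero input turns the sprite to face its direction by rotating it 180 degrees rather than mirroring its scale.
; The Jump action calls the built-in character jump.
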(event Input|ActionEvents|InputActionJump
  (params (Key :type Key%20Structure :default "None"))
  (:Pressed
    (Character|Jump)))

(event Input|AxisEvents|InputAxisHorizontalMovement
  (params (AxisValue :type Float%20%28single-precision%29))
  (Sprite|SetFlipbook (Variables|Default|GetSprite) (select (== AxisValue 0.0) "/Game/Art/Characters/Blank_Animations/Idle/blank_idle.blank_idle" "/Game/Art/Characters/Blank_Animations/Run/blank_run_FB.blank_run_FB"))
  (Pawn|Input|AddMovementInput "1.000000, 0, 0" AxisValue false)
  (if (!= AxisValue 0.0)
    (Transformation|SetRelativeRotation (Variables|Default|GetSprite) (Math|Rotator|SelectRotator "0,180.000000, 0" "0,0.000000, 0" (> AxisValue 0.0)) false false)))

(fn ConstructionScript)